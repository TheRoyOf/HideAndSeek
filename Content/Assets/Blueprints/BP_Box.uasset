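; BP_Box is a box actor that varies its appearance through its construction script.
; The construction script sets its static mesh to one of the first three entries in a Mesh array at random, then gives it a random yaw up to 180 degrees.
; BeginPlay only calls the parent, and the MeshId variable is unused.
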(event `self.ReceiveBeginPlay`
  (`parent.ReceiveBeginPlay`))

(fn `UserConstructionScript`
  (`parent.UserConstructionScript`)
  (`StaticMeshComponent.SetStaticMesh` (`self.StaticMesh`) (`|GetArrayItem` (`self.Mesh`) (`KismetMathLibrary.RandomIntegerInRange` 0 2)))
  (`SceneComponent.K2_SetWorldRotation` (`self.StaticMesh`) (`KismetMathLibrary.MakeRotator` 0.0 0.0 (`KismetMathLibrary.RandomFloatInRange` 0.0 180.0)) false false))