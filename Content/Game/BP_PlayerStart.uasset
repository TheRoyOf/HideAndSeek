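; BP_PlayerStart is a spawn point that creates a character only while it is unoccupied.
; On the server, the Box overlap events clear the Free flag when something enters and set it again when an overlap ends.
; SpawnCharacter spawns the given class at the actor's transform if Free is set, otherwise it prints a red on-screen error naming the spot.
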(event `self.Box.OnComponentBeginOverlap`
  (params (OverlappedComponent :type "PrimitiveComponent Object Reference") (OtherActor :type "Actor Object Reference") (OtherComp :type "PrimitiveComponent Object Reference") (OtherBodyIndex :type Integer) (bFromSweep :type Boolean) (SweepResult :type "HitResult Structure (by ref)"))
  (`/Engine/EditorBlueprintResources/ActorMacros.Switch Has Authority`
    (:`Authority`
      (set `self.Free` false))))

(event `self.Box.OnComponentEndOverlap`
  (params (OverlappedComponent :type "PrimitiveComponent Object Reference") (OtherActor :type "Actor Object Reference") (OtherComp :type "PrimitiveComponent Object Reference") (OtherBodyIndex :type Integer))
  (`/Engine/EditorBlueprintResources/ActorMacros.Switch Has Authority`
    (:`Authority`
      (set `self.Free` true))))

(fn `SpawnCharacter`
  (params (Class :type "Actor Class Reference"))
  (returns (ReturnValue :type "Actor Object Reference"))
  (if (`self.Free`)
    (bind _returnvalue (`|SpawnActorFromClass` Class (`self.GetTransform`) "Undefined" "OverrideRootScale" null null))
    (return _returnvalue)
    (else
      (`KismetSystemLibrary.PrintString` (`KismetStringLibrary.Concat_StrStr` "ERROR: " (`KismetSystemLibrary.GetDisplayName` self) " dont free!") true true (struct :`R` 1.0 :`A` 1.0) 5.0))))

(fn `UserConstructionScript`)