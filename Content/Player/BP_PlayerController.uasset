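; Player controller for a networked seeker-versus-hider game, bridging BP_GameMode and the local BP_Hud lobby and player list.
; On authority it binds game mode dispatchers and registers itself, relaying timer, player list and stage updates through owning-client events.
; Team choice and start countdown requests go back through server events.
; Tab shows the player list during the Game stage; death hides role HUDs, but the server respawn call is unwired.
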(event `self.ReceiveBeginPlay`
  (`/Engine/EditorBlueprintResources/ActorMacros.Switch Has Authority`
    (:`Authority`
      (bind _asbp_game_mode (cast `/Game/Game/BP_GameMode` (`GameplayStatics.GetGameMode`)))
      (add `/Game/Game/BP_GameMode.UpdateStartGameTimer` _asbp_game_mode (delegate `UpdateStartGameTimer`))
      (add `/Game/Game/BP_GameMode.D_UpdatePlayerList` _asbp_game_mode (delegate `UpgradePlayerList`))
      (add `/Game/Game/BP_GameMode.D_ConnectPlayer` _asbp_game_mode (delegate `ConnectPlayer`))
      (add `/Game/Game/BP_GameMode.D_DisconnectPlayer` _asbp_game_mode (delegate `DissconnectPlayer`))
      (add `/Game/Game/BP_GameMode.D_Start_StartTimer` _asbp_game_mode (delegate `Start_StartTimer`))
      (add `/Game/Game/BP_GameMode.D_Stop_StartTimer` _asbp_game_mode (delegate `Stop_StartTimer`))
      (add `/Game/Game/BP_GameMode.D_UpdateGameStage` _asbp_game_mode (delegate `UpdateGameStage`))
      (`/Game/Game/BP_GameMode.ConnectPlayer` _asbp_game_mode self))
    (:`Remote`
      (`/Game/Player/BP_Hud.ShowLobby` (cast `/Game/Player/BP_Hud` (`self.GetHUD`) :!pure true) true))))

(event `ConnectPlayer`
  (params (Controller :type "/Game/Player/BP_PlayerController Object Reference")))

(event `DissconnectPlayer`
  (params (Controller :type "/Game/Player/BP_PlayerController Object Reference")))

(event `OwningPlayer_Stop_StartTimer`
  (`/Game/Widgets/W_Lobby.Update Start Bnt` (`/Game/Player/BP_Hud.W_Lobby` (cast `/Game/Player/BP_Hud` (`self.GetHUD`) :!pure true)) true))

(event `Stop_StartTimer`
  (`self.OwningPlayer_Stop_StartTimer`))

(event `UpdateStartGameTimer`
  (params (Time :type "Float (double-precision)") (Active :type Boolean))
  (`self.OwningPlayer_UpgradeStartTimerDelay` Time Active))

(event `UpgradePlayerList`
  (params (Players :type "Array of String (by ref)") (Roles :type "Array of /Game/Enums/E_Roles Enum (by ref)"))
  (`self.OwningClient_UpdatePlayerList` Players Roles))

(event `Start_StartTimer`
  (`self.OwningPlayer_Start_StartTimer`))

(event `UpdateGameStage`
  (params (GameState :type "/Game/Enums/E_GameStage Enum" :default "NewEnumerator0"))
  (`self.OwningPlayer_UpdateGameStage` GameState))

(event `OwningPlayer_Start_StartTimer`
  (`/Game/Widgets/W_Lobby.Update Start Bnt` (`/Game/Player/BP_Hud.W_Lobby` (cast `/Game/Player/BP_Hud` (`self.GetHUD`) :!pure true)) false))

(event `OwningPlayer_UpgradeStartTimerDelay`
  (params (Time :type "Float (double-precision)") (Active :type Boolean))
  (`/Game/Widgets/W_Lobby.UpdateTimer` (`/Game/Player/BP_Hud.W_Lobby` (cast `/Game/Player/BP_Hud` (`self.GetHUD`) :!pure true)) Time Active))

(event `OwningClient_UpdatePlayerList`
  (params (Players :type "Array of String") (E_Roles :type "Array of /Game/Enums/E_Roles Enum"))
  (bind _asbp_hud (cast `/Game/Player/BP_Hud` (`self.GetHUD`) :!pure true))
  (bind _w_lobby (`/Game/Player/BP_Hud.W_Lobby` _asbp_hud))
  (`/Engine/EditorBlueprintResources/StandardMacros.IsValid` _w_lobby
    (:`Is Valid`
      (`/Game/Player/BP_Hud.SetPlayerList` _asbp_hud Players E_Roles)
      (`/Game/Widgets/W_Lobby.UpdatePlayerList` _w_lobby Players E_Roles))))

(event `OwningPlayer_ShowLobby`
  (params (Show :type Boolean))
  (`/Game/Player/BP_Hud.ShowLobby` (cast `/Game/Player/BP_Hud` (`self.GetHUD`) :!pure true) Show))

(event `self.ReceiveDestroyed`
  (`/Engine/EditorBlueprintResources/ActorMacros.Switch Has Authority`
    (:`Authority`
      (bind _asbp_game_mode (cast `/Game/Game/BP_GameMode` (`GameplayStatics.GetGameMode`)))
      (`/Game/Game/BP_GameMode.DisconnectPlayer` _asbp_game_mode self))))

(event `PlayerDied`
  (bind _asbp_hud (cast `/Game/Player/BP_Hud` (`self.GetHUD`)))
  (`/Game/Player/BP_Hud.ShowSeekerHUD` _asbp_hud false)
  (`/Game/Player/BP_Hud.ShowHiderHUD` _asbp_hud false))

(event `SetTeam`
  (params (NewTeam :type "/Game/Enums/E_Roles Enum (by ref)"))
  (`self.Server_SetTeam` NewTeam))

(event `Server_SetTeam`
  (params (NewTeam :type "/Game/Enums/E_Roles Enum" :default "NewEnumerator1"))
  (`/Game/Game/BP_GameMode.SetPlayerTeam` (cast `/Game/Game/BP_GameMode` (`GameplayStatics.GetGameMode`) :!pure true) self NewTeam))

(event `Start_StartGame`
  (`self.Server_Start_StartGame`))

(event `Server_Start_StartGame`
  (`/Game/Game/BP_GameMode.CouldownStartGame` (cast `/Game/Game/BP_GameMode` (`GameplayStatics.GetGameMode`) :!pure true)))

(event `Server_PlayerDied`
  (bind _asbp_game_mode (cast `/Game/Game/BP_GameMode` (`GameplayStatics.GetGameMode`)))
  (`/Game/Game/BP_GameMode.RespawnPlayer` _asbp_game_mode self))

(event `Stop_StartGame`
  (`self.Server_Stop_StartGame`))

(event `Server_Stop_StartGame`
  (`/Game/Game/BP_GameMode.ResetCouldownStartGame` (cast `/Game/Game/BP_GameMode` (`GameplayStatics.GetGameMode`) :!pure true)))

(event `OwningPlayer_UpdateGameStage`
  (params (GameStage :type "/Game/Enums/E_GameStage Enum" :default "NewEnumerator0"))
  (set `self.GameStage` GameStage))

(event `Key|Tab`
  (params (Key :type "Key Structure"))
  (bind _asbp_hud (cast `/Game/Player/BP_Hud` (`self.GetHUD`) :!pure true))
  (:`Pressed`
    (switch `/Game/Enums/E_GameStage` (`self.GameStage`)
      (:`NewEnumerator1`
        (`/Game/Player/BP_Hud.ShowPlayerList` _asbp_hud true))))
  (:`Released`
    (switch `/Game/Enums/E_GameStage` (`self.GameStage`)
      (:`NewEnumerator1`
        (`/Game/Player/BP_Hud.ShowPlayerList` _asbp_hud false)))))

(event `OwningClient_ShowPlayerList`
  (bind _asbp_hud (cast `/Game/Player/BP_Hud` (`self.GetHUD`)))
  (`/Game/Player/BP_Hud.ShowPlayerList` _asbp_hud true))

(fn `UserConstructionScript`)