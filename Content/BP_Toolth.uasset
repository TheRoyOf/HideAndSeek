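; BP_Toolth is a utility Blueprint that reports how many Hider and Seeker spawn points exist in the level.
; SpawnPointCounts gathers all BP_PlayerStart actors and tallies them by their Roles value.
; The SpawnPointCount event calls that function and prints both totals on screen in red.
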(event `SpawnPointCount`
  (bind (_hider _seeker) (`self.SpawnPointCounts`))
  (`KismetSystemLibrary.PrintString` (`KismetStringLibrary.Concat_StrStr` "Hider " (`KismetStringLibrary.Conv_IntToString` _hider) " Seeker " (`KismetStringLibrary.Conv_IntToString` _seeker)) true true (struct :`R` 1.0 :`A` 1.0) 10.0))

(fn `SpawnPointCounts`
  (returns (Hider :type Integer) (Seeker :type Integer))
  (locals (l_Hider :type Integer :default 0) (l_Seeker :type Integer :default 0))
  (bind _outactors (`GameplayStatics.GetAllActorsOfClass` "/Game/Game/BP_PlayerStart.BP_PlayerStart_C"))
  (for _array_element _outactors
    (switch `/Game/Enums/E_Roles` (`/Game/Game/BP_PlayerStart.Roles` _array_element)
      (:`NewEnumerator1`
        (`/Engine/EditorBlueprintResources/StandardMacros.IncrementInt` (`local.l_Hider`)))
      (:`NewEnumerator2`
        (`/Engine/EditorBlueprintResources/StandardMacros.IncrementInt` (`local.l_Seeker`)))))
  (return (`local.l_Hider`) (`local.l_Seeker`)))

(fn `UserConstructionScript`)